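; Anim notify that toggles combat mode on the AI behaviors component of the character playing the animation.
; It acts only when the mesh owner is a locally controlled Character with a valid BP_AIBehaviorsComponent.
; It flips the current state through SetCombatMode rather than setting an explicit value, so each trigger reverses the mode.
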(fn `GetDefaultTriggerWeightThreshold`
  (returns (ReturnValue :type "Float (single-precision)"))
  (return 0.0))

(fn `Received_Notify`
  (params (MeshComp :type "SkeletalMeshComponent Object Reference") (Animation :type "AnimSequenceBase Object Reference") (EventReference :type "AnimNotifyEventReference Structure (by ref)"))
  (returns (ReturnValue :type Boolean))
  (bind _ascharacter (cast `Character` (`ActorComponent.GetOwner` MeshComp)))
  (if (`Pawn.IsLocallyControlled` _ascharacter)
    (bind _returnvalue (`Actor.GetComponentByClass` _ascharacter "/Game/_HiepVu_B0ss/_SourcePackage/AIBehaviorSystem/Blueprint/Component/BP_AIBehaviorsComponent.BP_AIBehaviorsComponent_C"))
    (`/Engine/EditorBlueprintResources/StandardMacros.IsValid` _returnvalue
      (:`Is Valid`
        (`/Game/_HiepVu_B0ss/_SourcePackage/AIBehaviorSystem/Blueprint/Component/BP_AIBehaviorsComponent.SetCombatMode` _returnvalue (select `bool` (`/Game/_HiepVu_B0ss/_SourcePackage/AIBehaviorSystem/Blueprint/Component/BP_AIBehaviorsComponent.IsInCombatMode?` _returnvalue) :`false` true))
        (return false)))))