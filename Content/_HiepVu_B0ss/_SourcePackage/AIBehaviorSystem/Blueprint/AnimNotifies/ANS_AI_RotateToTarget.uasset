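; Anim notify state, shown as "AI Rotate To Target", that makes an AI character turn toward the player during a window of an animation.
; On begin, it tells the owning BP_AI_Base to start rotating at the notify's interp speed; on end, it tells it to stop.
; Both calls run only when the AI is locally controlled and has a BP_AIBehaviorsComponent.
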(fn `GetNotifyName`
  (returns (ReturnValue :type String))
  (return "AI Rotate To Target"))

(fn `Received_NotifyBegin`
  (params (MeshComp :type "SkeletalMeshComponent Object Reference") (Animation :type "AnimSequenceBase Object Reference") (TotalDuration :type "Float (single-precision)") (EventReference :type "AnimNotifyEventReference Structure (by ref)"))
  (returns (ReturnValue :type Boolean))
  (bind _asbp_ai_base (cast `/Game/_HiepVu_B0ss/_SourcePackage/AIBehaviorSystem/Blueprint/AI/BP_AI_Base` (`ActorComponent.GetOwner` MeshComp)))
  (if (`Pawn.IsLocallyControlled` _asbp_ai_base)
    (`/Engine/EditorBlueprintResources/StandardMacros.IsValid` (`Actor.GetComponentByClass` _asbp_ai_base "/Game/_HiepVu_B0ss/_SourcePackage/AIBehaviorSystem/Blueprint/Component/BP_AIBehaviorsComponent.BP_AIBehaviorsComponent_C")
      (:`Is Valid`
        (`/Game/_HiepVu_B0ss/_SourcePackage/AIBehaviorSystem/Blueprint/AI/BP_AI_Base.StartRotateToPlayer` _asbp_ai_base (`self.Interp Speed Rotation`))
        (return true))
      (:`Is Not Valid`
        (return false)))))

(fn `Received_NotifyEnd`
  (params (MeshComp :type "SkeletalMeshComponent Object Reference") (Animation :type "AnimSequenceBase Object Reference") (EventReference :type "AnimNotifyEventReference Structure (by ref)"))
  (returns (ReturnValue :type Boolean))
  (bind _asbp_ai_base (cast `/Game/_HiepVu_B0ss/_SourcePackage/AIBehaviorSystem/Blueprint/AI/BP_AI_Base` (`ActorComponent.GetOwner` MeshComp)))
  (if (`Pawn.IsLocallyControlled` _asbp_ai_base)
    (`/Engine/EditorBlueprintResources/StandardMacros.IsValid` (`Actor.GetComponentByClass` _asbp_ai_base "/Game/_HiepVu_B0ss/_SourcePackage/AIBehaviorSystem/Blueprint/Component/BP_AIBehaviorsComponent.BP_AIBehaviorsComponent_C")
      (:`Is Valid`
        (`/Game/_HiepVu_B0ss/_SourcePackage/AIBehaviorSystem/Blueprint/AI/BP_AI_Base.StopRotateToPlayer` _asbp_ai_base)
        (return true))
      (:`Is Not Valid`
        (return false)))))