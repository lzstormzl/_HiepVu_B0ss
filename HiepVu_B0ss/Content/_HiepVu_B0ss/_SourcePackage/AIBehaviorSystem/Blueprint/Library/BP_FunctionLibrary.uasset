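; Blueprint function library for the AI behavior system with one helper, GetHitDirection, which classifies where a hit on an actor comes from.
; It negates the hit direction and compares it with the actor's forward vector on the horizontal plane, using angle thresholds for a narrow front cone and a wider rear arc.
; Remaining hits split by the right-vector dot product, returning a four-way enum that defaults to front for an invalid actor.
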(fn `GetHitDirection`
  (params (HitFromDirection :type "Vector Structure") (AttackedActor :type "Actor Object Reference"))
  (returns (Direction :type "/Game/_HiepVu_B0ss/_SourcePackage/AIBehaviorSystem/Blueprint/Enums/E_HitDirection Enum"))
  (locals (L_HitNormal :type "Vector Structure" :default (0.0 0.0 0.0)) (L_AngleToHitNormal :type "Float (double-precision)" :default 0.0))
  (bind _l_angletohitnormal (`local.L_AngleToHitNormal`))
  (set `local.L_HitNormal` (`KismetMathLibrary.NegateVector` HitFromDirection))
  (`/Engine/EditorBlueprintResources/StandardMacros.IsValid` AttackedActor
    (:`Is Valid`
      (set `local.L_AngleToHitNormal` (`KismetMathLibrary.DegAcos` (`KismetMathLibrary.Dot_VectorVector` (`KismetMathLibrary.Vector_Normal2D` (`Actor.GetActorForwardVector` (`local.AttackedActor`))) (`KismetMathLibrary.Vector_Normal2D` (`local.L_HitNormal`)))))
      (`|ExecutionSequence`
        (:`then_0`
          (if (<= _l_angletohitnormal 25.0)
            (return "NewEnumerator0")))
        (:`then_1`
          (if (>= _l_angletohitnormal 135.0)
            (return "NewEnumerator2")))
        (:`then_2`
          (if (>= (`KismetMathLibrary.Dot_VectorVector` (`KismetMathLibrary.Vector_Normal2D` (`Actor.GetActorRightVector` (`local.AttackedActor`))) (`KismetMathLibrary.Vector_Normal2D` (`local.L_HitNormal`))) 0.0)
            (return "NewEnumerator3")
            (else
              (return "NewEnumerator1"))))))
    (:`Is Not Valid`
      (return "NewEnumerator0"))))