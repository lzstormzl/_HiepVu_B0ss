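; BP_EnemyBase is the base enemy Blueprint, providing a sword-wielding attack.
; WieldSword spawns BP_SwordE, snaps it to the mesh's right-hand socket and sets a wielding flag.
; Attack plays a warrior montage and calls the OnAttackEnd dispatcher on completion or interruption.
; ChasePlayer is empty, and a move-to-player, attack, delay and repeat chain is left unconnected, so it never runs.
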(event `self.ReceiveBeginPlay`)

(event `ChasePlayer`)

(event `Attack`
  (`|PlayMontage` (`self.Mesh`) "/Game/_AI/Enemy/Anim/Anim_Warrior_Attack_1_Montage.Anim_Warrior_Attack_1_Montage"
    (:`OnCompleted`
      _)
    (:`OnInterrupted`
      _))
  (`self.OnAttackEnd`))

(event `WieldSword`
  (bind _returnvalue (`|SpawnActorFromClass` "/Game/_AI/Enemy/AI/BP_SwordE.BP_SwordE_C" (`self.GetTransform`) "Undefined" "MultiplyWithRoot" null null))
  (`self.K2_AttachToComponent` _returnvalue (`self.Mesh`) "riflehand_r" "SnapToTarget" "SnapToTarget" "KeepRelative" true)
  (set `self.IsWiedingSword` true))

(fn `UserConstructionScript`)